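; Player character Blueprint with a right-mouse melee attack driven by the AM_Boxing montage.
; An IsAttacking flag blocks re-triggering, and movement is disabled until the montage completes, then set back to walking.
; A montage notify fires a short forward sphere trace for pawns from AttackTrace with debug drawing; the hit result is not used.
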(event `Key|RightMouseButton`
  (params (Key :type "Key Structure"))
  (bind _attacktrace (`self.AttackTrace`))
  (bind _returnvalue (`SceneComponent.K2_GetComponentLocation` _attacktrace))
  (:`Pressed`
    (if (not (`self.isAttacking`))
      (`|PlayMontage` (`self.Mesh`) "/Game/Assets/Animations/AM_Boxing.AM_Boxing"
        (:`then`
          (set `self.isAttacking` true)
          (`CharacterMovementComponent.DisableMovement` (`self.CharacterMovement`)))
        (:`OnCompleted`
          (set `self.isAttacking` false)
          (`CharacterMovementComponent.SetMovementMode` (`self.CharacterMovement`) "MOVE_Walking" 0))
        (:`OnNotifyBegin`
          (`KismetSystemLibrary.SphereTraceSingleForObjects` :`Start` _returnvalue :`End` (+ _returnvalue (* (`KismetMathLibrary.GetForwardVector` (`SceneComponent.K2_GetComponentRotation` _attacktrace)) 100.0)) :`Radius` 25.0 :`ObjectTypes` (`|MakeArray` "ObjectTypeQuery3" :!type "EObjectTypeQuery Enum") :`DrawDebugType` "ForDuration"))))))

(fn `UserConstructionScript`)