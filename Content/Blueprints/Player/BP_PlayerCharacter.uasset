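; Player character Blueprint with a boxing melee attack and selection of a current target.
; Right mouse starts the attack montage unless jumping or already attacking, disabling movement until the montage completes.
; A montage notify fires a debug-drawn sphere trace for pawns ahead of AttackTrace, though the hit result is unused.
; SetTarget moves the selected state between targets, marked for a move to C++ UnitCharacter.
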(event `Key|RightMouseButton`
  (params (Key :type "Key Structure"))
  (bind _attacktrace (`self.AttackTrace`))
  (bind _returnvalue (`SceneComponent.K2_GetComponentLocation` _attacktrace))
  ;[1 1 1] Attack action
  (:`Pressed`
    (if (not (or (`self.IsJumping`) (`self.isAttacking`)))
      (`|PlayMontage` (`self.Mesh`) "/Game/Assets/Animations/AM_Boxing.AM_Boxing"
        (:`then`
          (set `self.isAttacking` true)
          (`CharacterMovementComponent.DisableMovement` (`self.CharacterMovement`)))
        (:`OnCompleted`
          (set `self.isAttacking` false)
          (`CharacterMovementComponent.SetMovementMode` (`self.CharacterMovement`) "MOVE_Walking" 0))
        (:`OnNotifyBegin`
          (`KismetSystemLibrary.SphereTraceSingleForObjects` :`Start` _returnvalue :`End` (+ _returnvalue (* (`KismetMathLibrary.GetForwardVector` (`SceneComponent.K2_GetComponentRotation` _attacktrace)) 100.0)) :`Radius` 25.0 :`ObjectTypes` (`|MakeArray` "ObjectTypeQuery3" :!type "EObjectTypeQuery Enum") :`DrawDebugType` "ForDuration"))))))

(fn `SetTarget`
  (params (NewTarget :type "/Game/Blueprints/Unit/BP_UnitCharacter Object Reference"))
  (bind _currenttarget (`self.CurrentTarget`))
  ;[1 1 1] @TODO: Should be move to Cpp in UnitCharacter to avoid a duplication with Unit targeting
  (`/Engine/EditorBlueprintResources/StandardMacros.IsValid` _currenttarget
    (:`Is Valid`
      (if (not (== _currenttarget NewTarget))
        (`/Game/Blueprints/Unit/BP_UnitCharacter.IsSelected` (`self.CurrentTarget`) false)
        (bind _output_get (set `self.CurrentTarget` NewTarget))
        (`/Game/Blueprints/Unit/BP_UnitCharacter.IsSelected` _output_get true)))
    (:`Is Not Valid`
      (bind _output_get_2 (set `self.CurrentTarget` NewTarget))
      (`/Game/Blueprints/Unit/BP_UnitCharacter.IsSelected` _output_get_2 true))))

(fn `UserConstructionScript`)